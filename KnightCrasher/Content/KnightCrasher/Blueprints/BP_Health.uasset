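; BP_Health is a health pickup for the player's CH_Knight character.
; On any actor overlap it fetches player character 0 rather than checking the overlapping actor, and casts it to CH_Knight.
; If the knight's health differs from maximum, it adds HealthValue, caps the result at MaxHealth and destroys itself.
; At full health the pickup stays in the world.
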(event Collision|EventActorBeginOverlap
  (params (OtherActor :type Actor%20Object%20Reference))
  (bind _asch_knight (Utilities|Casting|CastToCH_Knight (Game|GetPlayerCharacter 0)))
  (if (not (== (Variables|/Game/KnightCrasher/Character/CH_Knight.CH_Knight_C|GetcurrentHealth _asch_knight) (Variables|/Game/KnightCrasher/Character/CH_Knight.CH_Knight_C|GetmaxHealth _asch_knight)))
    (Variables|/Game/KnightCrasher/Character/CH_Knight.CH_Knight_C|SetcurrentHealth _asch_knight (+ (Variables|/Game/KnightCrasher/Character/CH_Knight.CH_Knight_C|GetcurrentHealth _asch_knight) (Variables|Default|GethealthValue)))
    (if (> (Variables|/Game/KnightCrasher/Character/CH_Knight.CH_Knight_C|GetcurrentHealth _asch_knight) (Variables|/Game/KnightCrasher/Character/CH_Knight.CH_Knight_C|GetmaxHealth _asch_knight))
      (Variables|/Game/KnightCrasher/Character/CH_Knight.CH_Knight_C|SetcurrentHealth _asch_knight (Variables|/Game/KnightCrasher/Character/CH_Knight.CH_Knight_C|GetmaxHealth _asch_knight))
      (Actor|DestroyActor)
      (else
        (Actor|DestroyActor)))))

(fn ConstructionScript)